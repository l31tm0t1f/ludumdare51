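; BP_Sheer is a shears goal object that wins the game when the first-person player character overlaps its sphere.
; The overlap sets KeyCollected on the character and plays a success sound at the Shear component's location.
; After a short delay it shows the MessageWon widget, enables the mouse cursor and plays a second sound in 2D.
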(event OnComponentBeginOverlap(Sphere)
  (params (OverlappedComponent :type Primitive%20Component%20Object%20Reference) (OtherActor :type Actor%20Object%20Reference) (OtherComp :type Primitive%20Component%20Object%20Reference) (OtherBodyIndex :type Integer) (bFromSweep :type Boolean) (SweepResult :type Hit%20Result%20Structure%20%28by%20ref%29))
  (bind _asfirst_person_character_ld51 (Utilities|Casting|CastToFirstPersonCharacter_LD51 OtherActor))
  (Variables|/Game/LD51/FirstPersonCharacter_LD51.FirstPersonCharacter_LD51_C|SetKeyCollected? _asfirst_person_character_ld51 true)
  (Audio|PlaySoundatLocation "/Game/LD51/Sounds/magic-game-win-success-2.magic-game-win-success-2" (Transformation|GetWorldLocation (Variables|Default|GetShear)) "0, 0, 0" 1.0 1.0 0.0 0 0 0)
  (Utilities|FlowControl|Delay 2.0)
  (bind _returnvalue (UserInterface|CreateWidget "/Game/LD51/UI/MessageWon.MessageWon_C" 0 0 0))
  (UserInterface|Viewport|AddtoViewport _returnvalue 0)
  (Variables|/Script/Engine.PlayerController|SetbShowMouseCursor (Game|GetPlayerController 0) true)
  (Audio|PlaySound2D "/Game/LD51/Sounds/chopcjop.chopcjop" 1.0 1.0 0.0 0 0))

(event EventBeginPlay)

(event Collision|EventActorBeginOverlap
  (params (OtherActor :type Actor%20Object%20Reference)))

(event EventTick
  (params (DeltaSeconds :type Float%20%28single-precision%29)))

(fn ConstructionScript)