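; BP_Wall is a wall actor that rotates about its vertical axis once play begins.
; On BeginPlay it draws a random entry from Direction, and a value of 1 selects the RotateWall timeline, otherwise Timeline_0.
; The chosen timeline's vector track Z sets the root component's world yaw on each update, passing through its relative roll and pitch.
; A trailing Delay after each update leads to nothing.
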(event EventBeginPlay
  (bind _defaultsceneroot (Variables|Default|GetDefaultSceneRoot))
  (bind _defaultsceneroot_2 (Variables|Default|GetDefaultSceneRoot))
  (bind _relativerotation (Variables|/Script/Engine.SceneComponent|GetRelativeRotation _defaultsceneroot))
  (bind _relativerotation_2 (Variables|/Script/Engine.SceneComponent|GetRelativeRotation _defaultsceneroot_2))
  (if (== (.OutItem (Utilities|Array|Random (Variables|Default|GetDirection))) 1.0)
    (bind _newtrack_0 (Timeline|RotateWall Play)
      (:Update
        (Transformation|SetWorldRotation _defaultsceneroot_2 (Math|Rotator|MakeRotator (.roll _relativerotation_2) (.pitch _relativerotation_2) (.z _newtrack_0)) false false)
        (Utilities|FlowControl|Delay 1.0)))
    (else
      (bind _newtrack_0_2 (Timeline|Timeline_0 Play)
        (:Update
          (Transformation|SetWorldRotation _defaultsceneroot (Math|Rotator|MakeRotator (.roll _relativerotation) (.pitch _relativerotation) (.z _newtrack_0_2)) false false)
          (Utilities|FlowControl|Delay 1.0))))))

(event Collision|EventActorBeginOverlap
  (params (OtherActor :type Actor%20Object%20Reference)))

(event EventTick
  (params (DeltaSeconds :type Float%20%28single-precision%29)))

(fn ConstructionScript)